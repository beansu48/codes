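; BP_KeyToy is a spinning key in the maze area that updates the knight's task and unlocks a linked maze-in actor.
; Tick yaws the key mesh by a fixed, frame-rate-dependent step.
; The first box overlap by BP_Knight prints a debug message, sets the task box on the knight's main widget, then calls SetCanOpen on BPMazeIn if valid.
; A DoOnce limits this to one trigger, and the key stays in place.
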(event `self.ReceiveTick`
  (params (DeltaSeconds :type "Float (single-precision)"))
  (`SceneComponent.K2_AddRelativeRotation` (`self.SM_Key`) (`KismetMathLibrary.MakeRotator` 0.0 0.0 20.0) false false))

(event `self.Box.OnComponentBeginOverlap`
  (params (OverlappedComponent :type "PrimitiveComponent Object Reference") (OtherActor :type "Actor Object Reference") (OtherComp :type "PrimitiveComponent Object Reference") (OtherBodyIndex :type Integer) (bFromSweep :type Boolean) (SweepResult :type "HitResult Structure (by ref)"))
  (bind _bp_mazein (`self.BP_MazeIn`))
  (bind _asbp_knight (cast `/Game/Character/Knight/BP_Knight` OtherActor))
  (`/Engine/EditorBlueprintResources/StandardMacros.DoOnce` false
    (:`Completed`
      (`KismetSystemLibrary.PrintString` "Hello")
      (`/Game/UserInterface/Widgets/HUD/W_HUD_MainWidget.Set_TaskBox` (`/Game/Character/Knight/BP_Knight.MainWidget` _asbp_knight) (`self.TaskText`))
      (`/Engine/EditorBlueprintResources/StandardMacros.IsValid` _bp_mazein
        (:`Is Valid`
          (`/Game/Blueprints/MazeIn/BP_MazeIn.SetCanOpen` _bp_mazein))))))

(fn `UserConstructionScript`)