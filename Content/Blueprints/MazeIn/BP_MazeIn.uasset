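; BP_MazeIn is the entrance to the Labyrinth level, locked until SetCanOpen is called.
; A Sphere overlap by BP_Knight reveals a W_MazeInfo widget component, with no logic here to hide it again.
; A Box overlap by the knight loads the Labyrinth level if CanOpen is set.
; SetCanOpen sets that flag and copies it to the widget.
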(event `self.Box.OnComponentBeginOverlap`
  (params (OverlappedComponent :type "PrimitiveComponent Object Reference") (OtherActor :type "Actor Object Reference") (OtherComp :type "PrimitiveComponent Object Reference") (OtherBodyIndex :type Integer) (bFromSweep :type Boolean) (SweepResult :type "HitResult Structure (by ref)"))
  (cast `/Game/Character/Knight/BP_Knight` OtherActor)
  (if (`self.CanOpen`)
    (`GameplayStatics.OpenLevelBySoftObjectPtr` "/Game/Maps/labyrinth/labyrinth.labyrinth")))

(event `SetCanOpen`
  (set `self.CanOpen` true)
  (bind _asw_maze_info (cast `/Game/UserInterface/Widgets/MazeInfo/W_MazeInfo` (`WidgetComponent.GetUserWidgetObject` (`self.Widget`))))
  (set `/Game/UserInterface/Widgets/MazeInfo/W_MazeInfo.CanOpen` true _asw_maze_info))

(event `self.Sphere.OnComponentBeginOverlap`
  (params (OverlappedComponent :type "PrimitiveComponent Object Reference") (OtherActor :type "Actor Object Reference") (OtherComp :type "PrimitiveComponent Object Reference") (OtherBodyIndex :type Integer) (bFromSweep :type Boolean) (SweepResult :type "HitResult Structure (by ref)"))
  (cast `/Game/Character/Knight/BP_Knight` OtherActor)
  (`SceneComponent.SetVisibility` (`self.Widget`) true false))

(fn `UserConstructionScript`)