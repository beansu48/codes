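; Rockfall trap that spawns a limited number of BP_FallRock actors once a BP_Knight overlaps its TripBox.
; A looping timer spawns rocks at the height of RockSpawnPlane until RockCounter reaches RockNum, then clears itself.
; Spawn points blend random plane positions toward the player's XY, with a random-point fallback when the bounds check fails.
; Bounds derive from the plane's scale along world axes.
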(event `self.ReceiveBeginPlay`
  (bind (_returnvalue_x _returnvalue_y) (`KismetMathLibrary.BreakVector` (`SceneComponent.K2_GetComponentScale` (`self.RockSpawnPlane`))))
  (set `self.XRange` (* _returnvalue_x 50.0))
  (set `self.YRange` (* _returnvalue_y 50.0)))

(event `self.TripBox.OnComponentBeginOverlap`
  (params (OverlappedComponent :type "PrimitiveComponent Object Reference") (OtherActor :type "Actor Object Reference") (OtherComp :type "PrimitiveComponent Object Reference") (OtherBodyIndex :type Integer) (bFromSweep :type Boolean) (SweepResult :type "HitResult Structure (by ref)"))
  (cast `/Game/Character/Knight/BP_Knight` OtherActor)
  (bind _returnvalue (`KismetSystemLibrary.K2_SetTimerDelegate` (delegate `SpawnRockfall`) (`self.SpawnDelta`) true))
  (set `self.SpawnHandle` _returnvalue))

(event `SpawnRockfall`
  (bind _xrange (`self.XRange`))
  (bind _yrange (`self.YRange`))
  (bind _xrange_2 (`self.XRange`))
  (bind _yrange_2 (`self.YRange`))
  (bind (_returnvalue_x _returnvalue_y _returnvalue_z) (`KismetMathLibrary.BreakVector` (`SceneComponent.K2_GetComponentLocation` (`self.RockSpawnPlane`))))
  (bind (_returnvalue_x_2 _returnvalue_y_2) (`KismetMathLibrary.BreakVector` (`self.K2_GetActorLocation` (`GameplayStatics.GetPlayerCharacter` 0))))
  (bind (_returnvalue_x_3 _returnvalue_y_3) (`KismetMathLibrary.BreakVector` (`SceneComponent.K2_GetComponentLocation` (`self.RockSpawnPlane`))))
  (bind _returnvalue (+ (`SceneComponent.K2_GetComponentLocation` (`self.RockSpawnPlane`)) (* (`KismetMathLibrary.Vector_Right`) (`KismetMathLibrary.RandomFloatInRange` (* _yrange_2 -1.0) _yrange_2)) (* (`KismetMathLibrary.Vector_Forward`) (`KismetMathLibrary.RandomFloatInRange` (* _xrange_2 -1.0) _xrange_2))))
  (bind _returnvalue_2 (`KismetMathLibrary.VLerp` _returnvalue (`KismetMathLibrary.MakeVector` _returnvalue_x_2 _returnvalue_y_2 _returnvalue_z) (`KismetMathLibrary.RandomFloatInRange` 0.5 1.0)))
  (if (< (`self.RockCounter`) (`self.RockNum`))
    (`/Engine/EditorBlueprintResources/StandardMacros.IncrementInt` (`self.RockCounter`)
      (:`  `
        (`|SpawnActorFromClass` "/Game/Blueprints/RockfallTrap/BP_FallRock.BP_FallRock_C" (`KismetMathLibrary.MakeTransform` (`KismetMathLibrary.SelectVector` _returnvalue_2 _returnvalue (and (`KismetMathLibrary.InRange_FloatFloat` (.x _returnvalue_2) (- _returnvalue_x_3 _xrange) (+ _returnvalue_x_3 _xrange)) (`KismetMathLibrary.InRange_FloatFloat` (.y _returnvalue_2) (- _returnvalue_y_3 _yrange) (+ _returnvalue_y_3 _yrange))))) "Undefined" "OverrideRootScale" null null)))
    (else
      (`KismetSystemLibrary.K2_ClearAndInvalidateTimerHandle` (`self.SpawnHandle`)))))

(fn `UserConstructionScript`)