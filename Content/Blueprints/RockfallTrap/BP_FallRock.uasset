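; BP_FallRock is a physics-driven falling rock hazard that marks where it will land.
; On BeginPlay it picks a random mesh from ChocolateRockLia, enables physics and traces downward, ignoring the player, to spawn a scaled BP_WarningRange at the hit point.
; The rock's first hit destroys that warning through a DoOnce, and only prints a debug message if it struck BP_Knight, with no damage applied.
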(event `self.ReceiveBeginPlay`
  (bind _chocolaterocklia (`self.ChocolateRockLia`))
  (`StaticMeshComponent.SetStaticMesh` (`self.SM_Rock`) (`|GetArrayItem` _chocolaterocklia (`KismetMathLibrary.RandomIntegerInRange` 0 (- (`KismetArrayLibrary.Array_Length` _chocolaterocklia) 1))))
  (`PrimitiveComponent.SetSimulatePhysics` (`self.SM_Rock`) true)
  (`self.SetWarningRange`))

(event `SetWarningRange`
  (bind _returnvalue (`SceneComponent.K2_GetComponentLocation` (`self.SM_Rock`)))
  (bind (_outhit _returnvalue_2) (`KismetSystemLibrary.LineTraceSingle` _returnvalue (+ _returnvalue (* (`KismetMathLibrary.Vector_Down`) (`self.WarningDistance`))) "TraceTypeQuery2" false (`|MakeArray` (`GameplayStatics.GetPlayerCharacter` 0) :!type "Actor Object Reference")))
  (if _returnvalue_2
    (bind _returnvalue_3 (`|SpawnActorFromClass` "/Game/Blueprints/RockfallTrap/BP_WarningRange.BP_WarningRange_C" (`KismetMathLibrary.MakeTransform` (`.Location` (`GameplayStatics.BreakHitResult` _outhit)) (struct) (* (`SceneComponent.K2_GetComponentScale` (`self.SM_Rock`)) 2.0)) "AlwaysSpawn" "OverrideRootScale" null null))
    (set `self.WarningRange` _returnvalue_3)))

(event `self.SM_Rock.OnComponentHit`
  (params (HitComponent :type "PrimitiveComponent Object Reference") (OtherActor :type "Actor Object Reference") (OtherComp :type "PrimitiveComponent Object Reference") (NormalImpulse :type "Vector Structure") (Hit :type "HitResult Structure (by ref)"))
  (`/Engine/EditorBlueprintResources/StandardMacros.DoOnce` false
    (:`Completed`
      (cast `/Game/Character/Knight/BP_Knight` OtherActor
        (:`then`
          (`KismetSystemLibrary.PrintString` "Player Hit!"))
        (:`CastFailed`
          _))
      (`self.K2_DestroyActor` (`self.WarningRange`)))))

(fn `UserConstructionScript`)