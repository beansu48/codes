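; BP_SlipRope is a zipline-style rope that carries a BP_Knight along the direction of its Arrow component.
; Entering the box switches the knight to Flying, stops its movement and aligns its rotation with the arrow.
; While the knight is inside, Tick moves it forward with a swept offset at Speed.
; Leaving the box restores Walking and adds a forward velocity-change impulse of twice Speed to launch it off.
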(event `self.BoxCollision.OnComponentBeginOverlap`
  (params (OverlappedComponent :type "PrimitiveComponent Object Reference") (OtherActor :type "Actor Object Reference") (OtherComp :type "PrimitiveComponent Object Reference") (OtherBodyIndex :type Integer) (bFromSweep :type Boolean) (SweepResult :type "HitResult Structure (by ref)"))
  (bind _asbp_knight (cast `/Game/Character/Knight/BP_Knight` OtherActor))
  (set `self.Knight` _asbp_knight)
  (set `self.KnightIn` true)
  (`CharacterMovementComponent.SetMovementMode` (`Character.CharacterMovement` (`self.Knight`)) "MOVE_Flying" 0)
  (`MovementComponent.StopMovementImmediately` (`Character.CharacterMovement` (`self.Knight`)))
  (`self.K2_SetActorRotation` (`self.Knight`) (`SceneComponent.K2_GetComponentRotation` (`self.Arrow`)) false))

(event `self.BoxCollision.OnComponentEndOverlap`
  (params (OverlappedComponent :type "PrimitiveComponent Object Reference") (OtherActor :type "Actor Object Reference") (OtherComp :type "PrimitiveComponent Object Reference") (OtherBodyIndex :type Integer))
  (cast `/Game/Character/Knight/BP_Knight` OtherActor)
  (set `self.KnightIn` false)
  (`CharacterMovementComponent.SetMovementMode` (`Character.CharacterMovement` (`self.Knight`)) "MOVE_Walking" 0)
  (`CharacterMovementComponent.AddImpulse` (`Character.CharacterMovement` (`self.Knight`)) (* (`SceneComponent.GetForwardVector` (`self.Arrow`)) (* 2 (`self.Speed`))) true))

(event `self.ReceiveTick`
  (params (DeltaSeconds :type "Float (single-precision)"))
  (if (`self.KnightIn`)
    (`/Engine/EditorBlueprintResources/StandardMacros.IsValid` (`self.Knight`)
      (:`Is Valid`
        (`self.K2_AddActorWorldOffset` (`self.Knight`) (* (`SceneComponent.GetForwardVector` (`self.Arrow`)) (* DeltaSeconds (`self.Speed`))) true true)))))

(fn `UserConstructionScript`)