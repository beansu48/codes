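; BP_QTEDoor is a door that the knight opens by succeeding at a quick-time event.
; While the door is closed, overlapping its box creates a W_QTE widget in the knight's main HUD, and leaving the box removes it.
; The widget's success event triggers a one-time OpenDoor, where a timeline swings the mesh a quarter turn from its starting yaw, removes the widget and flags the door open.
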(event `self.BoxCollision.OnComponentBeginOverlap`
  (params (OverlappedComponent :type "PrimitiveComponent Object Reference") (OtherActor :type "Actor Object Reference") (OtherComp :type "PrimitiveComponent Object Reference") (OtherBodyIndex :type Integer) (bFromSweep :type Boolean) (SweepResult :type "HitResult Structure (by ref)"))
  (bind _asbp_knight (cast `/Game/Character/Knight/BP_Knight` OtherActor))
  (set `self.BP Knight` _asbp_knight)
  (if (not (`self.IsDoorOpen`))
    (bind _returnvalue (`|CreateWidget` "/Game/UserInterface/Widgets/QTE/W_QTE.W_QTE_C" (`GameplayStatics.GetPlayerController` 0)))
    (bind _output_get (set `self.W_QTE` _returnvalue))
    (`/Game/UserInterface/Widgets/HUD/W_HUD_MainWidget.AddWidgetToMidDownBox` (`/Game/Character/Knight/BP_Knight.MainWidget` (`self.BP Knight`)) _output_get)
    (add `/Game/UserInterface/Widgets/QTE/W_QTE.QTE_Success` (`self.W_QTE`) (delegate `Open Door`))))

(event `self.BoxCollision.OnComponentEndOverlap`
  (params (OverlappedComponent :type "PrimitiveComponent Object Reference") (OtherActor :type "Actor Object Reference") (OtherComp :type "PrimitiveComponent Object Reference") (OtherBodyIndex :type Integer))
  (bind _asbp_knight (cast `/Game/Character/Knight/BP_Knight` OtherActor))
  (set `self.BP Knight` _asbp_knight)
  (`/Game/UserInterface/Widgets/HUD/W_HUD_MainWidget.RemoveWidgetOnMidDownBox` (`/Game/Character/Knight/BP_Knight.MainWidget` (`self.BP Knight`)) (`self.W_QTE`)))

(event `Open Door`
  (bind (_returnvalue_roll _returnvalue_pitch _returnvalue_yaw) (`KismetMathLibrary.BreakRotator` (`SceneComponent.K2_GetComponentRotation` (`self.SM_Door`))))
  (bind (_returnvalue_roll_2 _returnvalue_pitch_2) (`KismetMathLibrary.BreakRotator` (`SceneComponent.K2_GetComponentRotation` (`self.SM_Door`))))
  (`/Engine/EditorBlueprintResources/StandardMacros.DoOnce` false
    (:`Completed`
      (set `self.RawYaw` _returnvalue_yaw)
      (bind (_direction _rotation) (`Timeline|Rotation` :!via `PlayFromStart`)
        (:`Update`
          (`SceneComponent.K2_SetWorldRotation` (`self.SM_Door`) (`KismetMathLibrary.MakeRotator` _returnvalue_roll_2 _returnvalue_pitch_2 (+ (`KismetMathLibrary.Lerp` 0.0 -90.0 _rotation) (`self.RawYaw`))) false false)
          (`/Game/UserInterface/Widgets/HUD/W_HUD_MainWidget.RemoveWidgetOnMidDownBox` (`/Game/Character/Knight/BP_Knight.MainWidget` (`self.BP Knight`)) (`self.W_QTE`))
          (set `self.IsDoorOpen` true))))))

(fn `UserConstructionScript`)