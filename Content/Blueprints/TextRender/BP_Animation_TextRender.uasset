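; Animated text actor that builds a string from one BP_Animation_WordRender child actor per character and animates it in and out.
; The construction script rebuilds the characters along Y, spacing them by text world size and treating "*" as a line break.
; Show staggers fade, rotate, move and grow animations with a retriggerable-delay loop, then calls ShowFinished.
; Remove triggers the reverse animations on all characters at once and calls OutFinished immediately.
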(event `Remove`
  (for _array_element (`self.WordRenders`)
    (`/Game/Blueprints/TextRender/BP_Animation_WordRender.FadeOut` _array_element)
    (`/Game/Blueprints/TextRender/BP_Animation_WordRender.Rotate` _array_element)
    (`/Game/Blueprints/TextRender/BP_Animation_WordRender.MoveOut` _array_element)
    (`/Game/Blueprints/TextRender/BP_Animation_WordRender.Narrow` _array_element))
  (`self.OutFinished`))

(event `Show`
  (bind _output (`|GetArrayItem` (`self.WordRenders`) (`self.count`)))
  (set `self.count` 0)
  (if (< (`self.count`) (`KismetArrayLibrary.Array_Length` (`self.WordRenders`))) :!label _label
    (`/Game/Blueprints/TextRender/BP_Animation_WordRender.FadeIn` _output)
    (`/Game/Blueprints/TextRender/BP_Animation_WordRender.RotateBack` _output)
    (`/Game/Blueprints/TextRender/BP_Animation_WordRender.MoveBack` _output)
    (`/Game/Blueprints/TextRender/BP_Animation_WordRender.Grow` _output)
    (`/Engine/EditorBlueprintResources/StandardMacros.IncrementInt` (`self.count`)
      (:`  `
        (`KismetSystemLibrary.RetriggerableDelay` 0.2)
        (goto _label)))
    (else
      (`self.ShowFinished`))))

(fn `CreateText`
  (params (SourceString :type String))
  (bind (_location_x _location_y _location_z) (`KismetMathLibrary.BreakVector` (`self.Location`)))
  (bind (_location_x_2 _location_y_2 _location_z_2) (`KismetMathLibrary.BreakVector` (`self.Location`)))
  (for _array_element (`self.WordRenders`)
    (`self.K2_DestroyActor` _array_element))
  (`KismetArrayLibrary.Array_Clear` (`self.WordRenders`))
  (set `self.Location` (0.0 0.0 0.0))
  (for _array_element_2 (`KismetStringLibrary.GetCharacterArrayFromString` SourceString)
    (if (not (`KismetStringLibrary.EqualEqual_StrStr` _array_element_2 "*"))
      (bind _returnvalue (`AddComponent|NODE_AddChildActorComponent-1` :`self` self :`RelativeTransform` (`KismetMathLibrary.MakeTransform` (`self.Location`) (struct :`Yaw` 180.0))))
      (bind _asbp_animation_word_render (cast `/Game/Blueprints/TextRender/BP_Animation_WordRender` (`ChildActorComponent.ChildActor` _returnvalue)))
      (`KismetArrayLibrary.Array_Add` (`self.WordRenders`) _asbp_animation_word_render)
      (`|ExecutionSequence`
        (:`then_0`
          (bind (_returnvalue_x _returnvalue_y) (`KismetMathLibrary.BreakVector` (`TextRenderComponent.GetTextWorldSize` (`TextRenderActor.TextRender` _asbp_animation_word_render))))
          (set `self.Location` (`KismetMathLibrary.MakeVector` _location_x (+ (* 2 _returnvalue_y) _location_y) _location_z)))
        (:`then_1`
          (set `/Game/Blueprints/TextRender/BP_Animation_WordRender.Word` _array_element_2 _asbp_animation_word_render)
          (set `/Game/Blueprints/TextRender/BP_Animation_WordRender.Size` (`self.Size`) _asbp_animation_word_render)
          (`/Game/Blueprints/TextRender/BP_Animation_WordRender.DoSet` _asbp_animation_word_render)))
      (else
        (set `self.Location` (`KismetMathLibrary.MakeVector` _location_x_2 0.0 (+ -102.0 _location_z_2)))))))

(fn `UserConstructionScript`
  (locals (NewLocalVar_0 :type "Vector Structure" :default (0.0 0.0 0.0)))
  (`self.CreateText` (`self.Text`)))