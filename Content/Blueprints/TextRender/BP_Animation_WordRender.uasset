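; Text render actor that displays a configurable word and animates it through callable events.
; Construction and BeginPlay apply word and size; DoSet reruns the BeginPlay setup.
; Separate timelines drive paired effects: alpha fade in/out, size grow/narrow, random yaw spin and random-direction movement out/back.
; Back variants pick a fresh random offset and lerp from it to the transform captured at call time, rather than undoing the earlier motion.
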(event `self.ReceiveBeginPlay`
  (bind _textrender (`self.TextRender`))
  (bind (_textrendercolor_b _textrendercolor_g _textrendercolor_r) (break `Color` (`TextRenderComponent.TextRenderColor` _textrender)))
  (`TextRenderComponent.K2_SetText` (`self.TextRender`) (`KismetTextLibrary.Conv_StringToText` (`self.Word`)) :!label _label)
  (`TextRenderComponent.SetWorldSize` (`self.TextRender`) (`self.Size`))
  (`TextRenderComponent.SetTextRenderColor` _textrender (make `Color` _textrendercolor_b _textrendercolor_g _textrendercolor_r)))

(event `DoSet`
  (goto _label))

(event `FadeIn`
  (bind (_textrendercolor_b _textrendercolor_g _textrendercolor_r) (break `Color` (`TextRenderComponent.TextRenderColor` (`self.TextRender`))))
  (bind (_textrendercolor_b_2 _textrendercolor_g_2 _textrendercolor_r_2) (break `Color` (`TextRenderComponent.TextRenderColor` (`self.TextRender`))))
  ;[1 1 1] Set A  = 0
  (`TextRenderComponent.SetTextRenderColor` (`self.TextRender`) (make `Color` _textrendercolor_b _textrendercolor_g _textrendercolor_r))
  ;[1 1 1] Fade IN
  (bind (_direction _fade) (`Timeline|TFadeIn` :!via `PlayFromStart`)
    (:`Update`
      (`TextRenderComponent.SetTextRenderColor` (`self.TextRender`) (make `Color` _textrendercolor_b_2 _textrendercolor_g_2 _textrendercolor_r_2 (`KismetMathLibrary.Conv_Int64ToByte` (`KismetMathLibrary.FTrunc64` _fade)))))))

(event `FadeOut`
  (bind (_textrendercolor_b _textrendercolor_g _textrendercolor_r) (break `Color` (`TextRenderComponent.TextRenderColor` (`self.TextRender`))))
  (bind (_textrendercolor_b_2 _textrendercolor_g_2 _textrendercolor_r_2) (break `Color` (`TextRenderComponent.TextRenderColor` (`self.TextRender`))))
  ;[1 1 1] Set A  = 0
  (`TextRenderComponent.SetTextRenderColor` (`self.TextRender`) (make `Color` _textrendercolor_b_2 _textrendercolor_g_2 _textrendercolor_r_2))
  ;[1 1 1] Fade Out
  (bind (_direction _fade) (`Timeline|TFadeOut` :!via `PlayFromStart`)
    (:`Update`
      (`TextRenderComponent.SetTextRenderColor` (`self.TextRender`) (make `Color` _textrendercolor_b _textrendercolor_g _textrendercolor_r (`KismetMathLibrary.Conv_Int64ToByte` (`KismetMathLibrary.FTrunc64` _fade)))))))

(event `Rotate`
  (bind (_rawrotation_roll _rawrotation_pitch _rawrotation_yaw) (`KismetMathLibrary.BreakRotator` (`self.RawRotation`)))
  ;[1 1 1] 注释
  (set `self.RawRotation` (`self.K2_GetActorRotation`))
  (set `self.RotationFloat` (`KismetMathLibrary.RandomFloatInRange` 100.0 200.0))
  (bind (_direction _rotation) (`Timeline|TRotate` :!via `PlayFromStart`)
    (:`Update`
      (`self.K2_SetActorRotation` (`KismetMathLibrary.RLerp` (`self.RawRotation`) (`KismetMathLibrary.MakeRotator` (+ _rawrotation_roll 1.0) (+ _rawrotation_pitch 1.0) (+ _rawrotation_yaw (* 1 (`self.RotationFloat`)))) _rotation)))))

(event `RotateBack`
  (bind (_rawrotation_roll _rawrotation_pitch _rawrotation_yaw) (`KismetMathLibrary.BreakRotator` (`self.RawRotation`)))
  ;[1 1 1] 注释
  (set `self.RawRotation` (`self.K2_GetActorRotation`))
  (set `self.RotationFloat` (`KismetMathLibrary.RandomFloatInRange` 100.0 200.0))
  (bind (_direction _rotation) (`Timeline|TRotateBack` :!via `PlayFromStart`)
    (:`Update`
      (`self.K2_SetActorRotation` (`KismetMathLibrary.RLerp` (`KismetMathLibrary.MakeRotator` (+ _rawrotation_roll 1.0) (+ _rawrotation_pitch 1.0) (+ _rawrotation_yaw (* 1 (`self.RotationFloat`)))) (`self.RawRotation`) _rotation)))))

(event `Grow`
  ;[1 1 1] 注释
  (`TextRenderComponent.SetWorldSize` (`self.TextRender`) 0.0)
  (bind (_direction _size) (`Timeline|TGrow` :!via `PlayFromStart`)
    (:`Update`
      (`TextRenderComponent.SetWorldSize` (`self.TextRender`) (`KismetMathLibrary.Lerp` 0.0 (`self.Size`) _size)))))

(event `Narrow`
  ;[1 1 1] Narrow
  (`TextRenderComponent.SetWorldSize` (`self.TextRender`) (`self.Size`))
  (bind (_direction _size) (`Timeline|TNarrow` :!via `ReverseFromEnd`)
    (:`Update`
      (`TextRenderComponent.SetWorldSize` (`self.TextRender`) (`KismetMathLibrary.Lerp` 0.0 (`self.Size`) _size)))))

(event `MoveOut`
  (bind (_returnvalue_x _returnvalue_y) (`KismetMathLibrary.BreakVector` (`KismetMathLibrary.RandomUnitVector`)))
  ;[1 1 1] MoveOut
  (set `self.RawLocation` (`self.K2_GetActorLocation`))
  (set `self.MoveDir` (`KismetMathLibrary.MakeVector` _returnvalue_x _returnvalue_y 1.0))
  (bind (_direction _alpha) (`Timeline|TMoveOut` :!via `PlayFromStart`)
    (:`Update`
      (`self.K2_SetActorLocation` (`KismetMathLibrary.VLerp` (`self.RawLocation`) (+ (`self.RawLocation`) (* (`self.MoveDir`) (`self.MoveDistance`))) _alpha)))))

(event `MoveBack`
  (bind (_returnvalue_x _returnvalue_y) (`KismetMathLibrary.BreakVector` (`KismetMathLibrary.RandomUnitVector`)))
  ;[1 1 1] MoveBack
  (set `self.RawLocation` (`self.K2_GetActorLocation`))
  (set `self.MoveDir` (`KismetMathLibrary.MakeVector` _returnvalue_x _returnvalue_y 1.0))
  (bind (_direction _alpha) (`Timeline|TMoveBack` :!via `PlayFromStart`)
    (:`Update`
      (`self.K2_SetActorLocation` (`KismetMathLibrary.VLerp` (+ (`self.RawLocation`) (* (`self.MoveDir`) (`self.MoveDistance`))) (`self.RawLocation`) _alpha)))))

(fn `UserConstructionScript`
  (`TextRenderComponent.K2_SetText` (`self.TextRender`) (`KismetTextLibrary.Conv_StringToText` (`self.Word`)))
  (`TextRenderComponent.SetWorldSize` (`self.TextRender`) (`self.Size`)))