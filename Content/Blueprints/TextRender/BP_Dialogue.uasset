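; BP_Dialogue is a trigger actor that plays a sequence of dialogue entries once when BP_Knight overlaps its box.
; It walks DialogueList by chaining each entry's show-finished event to removal and its out-finished event to incrementing Count and showing the next valid entry.
; The same trigger also calls AddSpeed on an optional Belt reference, right after starting the dialogue.
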(event `self.TrigerBox.OnComponentBeginOverlap`
  (params (OverlappedComponent :type "PrimitiveComponent Object Reference") (OtherActor :type "Actor Object Reference") (OtherComp :type "PrimitiveComponent Object Reference") (OtherBodyIndex :type Integer) (bFromSweep :type Boolean) (SweepResult :type "HitResult Structure (by ref)"))
  (cast `/Game/Character/Knight/BP_Knight` OtherActor)
  (`/Engine/EditorBlueprintResources/StandardMacros.DoOnce` false
    (:`Completed`
      (`|ExecutionSequence`
        (:`then_0`
          (`self.Dialogue`))
        (:`then_1`
          (`/Engine/EditorBlueprintResources/StandardMacros.IsValid` (`self.Belt`)
            (:`Is Valid`
              (`/Game/Blueprints/ConveyorBelt/BP_ConveyorBelt.AddSpeed` (`self.Belt`)))))))))

(event `Dialogue`
  (bind _output (`|GetArrayItem` (`self.DialogueList`) (`self.count`)))
  (`/Engine/EditorBlueprintResources/StandardMacros.IsValid` _output
    (:`Is Valid`
      (add `/Game/Blueprints/TextRender/BP_Animation_TextRender.ShowFinished` _output (delegate `ShowFinished_Event`))
      (`/Game/Blueprints/TextRender/BP_Animation_TextRender.Show` _output))))

(event `ShowFinished_Event`
  (bind _output (`|GetArrayItem` (`self.DialogueList`) (`self.count`)))
  (add `/Game/Blueprints/TextRender/BP_Animation_TextRender.OutFinished` _output (delegate `OutFinished_Event`))
  (`/Game/Blueprints/TextRender/BP_Animation_TextRender.Remove` _output))

(event `OutFinished_Event`
  (bind _result (`/Engine/EditorBlueprintResources/StandardMacros.IncrementInt` (`self.count`))
    (:`  `
      (`KismetSystemLibrary.PrintString` (`KismetStringLibrary.Conv_IntToString` _result))
      (`self.Dialogue`))))

(fn `UserConstructionScript`)