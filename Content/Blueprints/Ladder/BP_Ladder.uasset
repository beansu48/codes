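; Ladder actor that switches an overlapping BP_Knight into climbing while it is inside the Box trigger.
; On entry it sets Flying movement, passes the ArrowUp direction as LadderDir, stops orient-to-movement and saves, then tilts, the mesh rotation.
; On exit it restores Walking and orient-to-movement, launches the knight slightly upward and resets mesh pitch and yaw from the saved rotation, with zero roll.
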(event `self.Box.OnComponentBeginOverlap`
  (params (OverlappedComponent :type "PrimitiveComponent Object Reference") (OtherActor :type "Actor Object Reference") (OtherComp :type "PrimitiveComponent Object Reference") (OtherBodyIndex :type Integer) (bFromSweep :type Boolean) (SweepResult :type "HitResult Structure (by ref)"))
  (bind (_returnvalue_roll _returnvalue_pitch _returnvalue_yaw) (`KismetMathLibrary.BreakRotator` (`KismetMathLibrary.RotatorFromAxisAndAngle` (`SceneComponent.GetForwardVector` (`self.ArrowForward`)))))
  (bind _asbp_knight (cast `/Game/Character/Knight/BP_Knight` OtherActor))
  (set `self.Knight` _asbp_knight)
  (bind _charactermovement (`Character.CharacterMovement` _asbp_knight))
  (`CharacterMovementComponent.SetMovementMode` _charactermovement "MOVE_Flying" 0)
  (set `/Game/Character/Knight/BP_Knight.LadderDir` (`SceneComponent.GetForwardVector` (`self.ArrowUp`)) _asbp_knight)
  (set `CharacterMovementComponent.bOrientRotationToMovement` false _charactermovement)
  (set `self.RawRotation` (`SceneComponent.K2_GetComponentRotation` (`Character.Mesh` (`self.Knight`))))
  (`SceneComponent.K2_SetWorldRotation` (`Character.Mesh` (`self.Knight`)) (`KismetMathLibrary.MakeRotator` 12.0 _returnvalue_pitch (+ _returnvalue_yaw 90.0)) false false))

(event `self.Box.OnComponentEndOverlap`
  (params (OverlappedComponent :type "PrimitiveComponent Object Reference") (OtherActor :type "Actor Object Reference") (OtherComp :type "PrimitiveComponent Object Reference") (OtherBodyIndex :type Integer))
  (bind (_rawrotation_roll _rawrotation_pitch _rawrotation_yaw) (`KismetMathLibrary.BreakRotator` (`self.RawRotation`)))
  (bind _asbp_knight (cast `/Game/Character/Knight/BP_Knight` OtherActor))
  (bind _charactermovement (`Character.CharacterMovement` _asbp_knight))
  (`CharacterMovementComponent.SetMovementMode` _charactermovement "MOVE_Walking" 0)
  (`Character.LaunchCharacter` _asbp_knight (`KismetMathLibrary.MakeVector` 0.0 0.0 100.0) false true)
  (set `CharacterMovementComponent.bOrientRotationToMovement` true _charactermovement)
  (`SceneComponent.K2_SetWorldRotation` (`Character.Mesh` (`self.Knight`)) (`KismetMathLibrary.MakeRotator` 0.0 _rawrotation_pitch _rawrotation_yaw) false false))

(fn `UserConstructionScript`)