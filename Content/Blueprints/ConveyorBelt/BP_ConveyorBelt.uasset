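; BP_ConveyorBelt is a conveyor belt that pushes overlapping BP_Knight actors along its arrow's forward direction with a swept per-tick offset.
; A self-restarting timeline oscillates or ramps the speed between slow and quick bounds and shows it on a W_ConvertBeltSpeedShow widget.
; AddSpeed raises only the slow bound, then resets both bounds after a retriggerable delay.
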(event `self.ReceiveBeginPlay`
  (`self.SpeedChange`))

(event `SpeedChange`
  (bind (_direction _speed) (`Timeline|SpeedLine` :!via `PlayFromStart`)
    (:`Update`
      (bind _output_get (set `self.Speed` (`KismetMathLibrary.Lerp` (`self.SlowSpeed`) (`self.QuickSpeed`) _speed)))
      (bind _asw_convert_belt_speed_show (cast `/Game/UserInterface/Widgets/ConveyorBeltSpeedShow/W_ConvertBeltSpeedShow` (`WidgetComponent.GetUserWidgetObject` (`self.Widget`))))
      (set `/Game/UserInterface/Widgets/ConveyorBeltSpeedShow/W_ConvertBeltSpeedShow.Speed` _output_get _asw_convert_belt_speed_show))
    (:`Finished`
      (`self.SpeedChange`))))

(event `self.ReceiveTick`
  (params (DeltaSeconds :type "Float (single-precision)"))
  (for _array_element (`PrimitiveComponent.GetOverlappingActors` (`self.Box`) "/Game/Character/Knight/BP_Knight.BP_Knight_C")
    (`self.K2_AddActorWorldOffset` _array_element (* (`SceneComponent.GetForwardVector` (`self.Arrow`)) (* DeltaSeconds (`self.Speed`))) true true)))

(event `AddSpeed`
  (set `self.SlowSpeed` 1000.0)
  (set `self.SlowSpeed` 1000.0)
  (`KismetSystemLibrary.RetriggerableDelay` 10.0)
  (set `self.SlowSpeed` 200.0)
  (set `self.QuickSpeed` 700.0))

(fn `UserConstructionScript`)