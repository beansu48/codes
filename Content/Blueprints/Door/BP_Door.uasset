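; BP_Door is a door that gets knocked away when a BP_Knight actor hits it.
; The first such hit sets the door mesh to overlap Pawn and Camera channels, then applies a horizontal velocity-change impulse scaled by Force.
; The impulse points from the actor's location toward the hit point, and the whole actor is destroyed after a short delay.
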(event `self.SM_Door.OnComponentHit`
  (params (HitComponent :type "PrimitiveComponent Object Reference") (OtherActor :type "Actor Object Reference") (OtherComp :type "PrimitiveComponent Object Reference") (NormalImpulse :type "Vector Structure") (Hit :type "HitResult Structure (by ref)"))
  (bind (_returnvalue_x _returnvalue_y) (`KismetMathLibrary.BreakVector` (- Hit_Location (`self.K2_GetActorLocation`))))
  (cast `/Game/Character/Knight/BP_Knight` OtherActor)
  (`/Engine/EditorBlueprintResources/StandardMacros.DoOnce` false
    (:`Completed`
      (`PrimitiveComponent.SetCollisionResponseToChannel` (`self.SM_Door`) "ECC_Pawn" "ECR_Overlap")
      (`PrimitiveComponent.SetCollisionResponseToChannel` (`self.SM_Door`) "ECC_Camera" "ECR_Overlap")
      (`PrimitiveComponent.AddImpulse` (`self.SM_Door`) (* (`KismetMathLibrary.Normal` (`KismetMathLibrary.MakeVector` _returnvalue_x _returnvalue_y)) (`self.force`)) "None" true)
      (`KismetSystemLibrary.RetriggerableDelay` 3.0)
      (`self.K2_DestroyActor`))))

(fn `UserConstructionScript`)