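; BP_Soldier is an enemy guard that patrols target actors and kills the player knight if it keeps seeing them.
; PawnSensing halts movement and holds a sighting flag until a retriggerable delay expires, then patrol resumes through looping AIMoveTo calls.
; A timer at the sensing interval raises or lowers an alert counter, feeding the overhead alert widget, playing the player's danger animation and triggering death once past maximum.
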(event `self.PawnSensing.OnSeePawn`
  (params (Pawn :type "Pawn Object Reference"))
  (cast `/Game/Character/Knight/BP_Knight` Pawn)
  (set `self.CanSeePlayer` true)
  (`MovementComponent.StopMovementImmediately` (`self.CharacterMovement`))
  (`KismetSystemLibrary.RetriggerableDelay` (`PawnSensingComponent.SensingInterval` (`self.PawnSensing`)))
  (set `self.CanSeePlayer` false)
  (`self.SoldierMove`))

(event `self.ReceiveBeginPlay`
  (`KismetSystemLibrary.K2_SetTimerDelegate` (delegate `Seen`) (`PawnSensingComponent.SensingInterval` (`self.PawnSensing`)) true)
  (`self.SoldierMove`))

(event `Seen`
  (if (`self.CanSeePlayer`)
    (`|ExecutionSequence`
      (:`then_0`
        (bind _result (`/Engine/EditorBlueprintResources/StandardMacros.IncrementInt` (`self.AlertNum`))
          (:`  `
            (if (> _result (`self.MaxAlertNum`))
              (set `self.AlertNum` (`self.MaxAlertNum`))
              (`self.SetAlertPer`)
              (`/Engine/EditorBlueprintResources/StandardMacros.DoOnce` false
                (:`Completed`
                  (bind _asbp_knight (cast `/Game/Character/Knight/BP_Knight` (`GameplayStatics.GetPlayerCharacter` 0)))
                  (`/Game/Character/Knight/BP_Knight.Death` _asbp_knight)))
              (else
                (`self.SetAlertPer`))))))
      (:`then_1`
        (bind _asbp_knight_2 (cast `/Game/Character/Knight/BP_Knight` (`GameplayStatics.GetPlayerCharacter` 0)))
        (`/Game/UserInterface/Widgets/HUD/W_HUD_MainWidget.DangerAni` (`/Game/Character/Knight/BP_Knight.MainWidget` _asbp_knight_2))))
    (else
      (bind _result_2 (`/Engine/EditorBlueprintResources/StandardMacros.DecrementInt` (`self.AlertNum`))
        (:`  `
          (if (<= _result_2 0)
            (set `self.AlertNum` 0))
          (`self.SetAlertPer`))))))

(event `SetAlertPer`
  (bind _asw_alert (cast `/Game/UserInterface/Widgets/SoldierAlert/W_Alert` (`WidgetComponent.GetUserWidgetObject` (`self.Widget_Alert`))))
  (set `/Game/UserInterface/Widgets/SoldierAlert/W_Alert.AlertPer` (/ (`KismetMathLibrary.Conv_IntToDouble` (`self.AlertNum`)) (`KismetMathLibrary.Conv_IntToDouble` (`self.MaxAlertNum`))) _asw_alert))

(event `SoldierMove`
  (bind (_returnvalue_x _returnvalue_y _returnvalue_z) (`KismetMathLibrary.BreakVector` (`self.K2_GetActorLocation`)))
  (bind (_returnvalue_x_2 _returnvalue_y_2) (`KismetMathLibrary.BreakVector` (`self.K2_GetActorLocation` (`|GetArrayItem` (`self.TargetA`) (`self.MoveCount`)))))
  (`/Engine/EditorBlueprintResources/StandardMacros.IsValid` (`|GetArrayItem` (`self.TargetA`) (`self.MoveCount`))
    (:`Is Valid`
      _)
    (:`Is Not Valid`
      (set `self.MoveCount` 0)))
  (`|AIMoveTo` self (`KismetMathLibrary.MakeVector` _returnvalue_x_2 _returnvalue_y_2 _returnvalue_z) null
    (:`OnSuccess`
      (`/Engine/EditorBlueprintResources/StandardMacros.IncrementInt` (`self.MoveCount`)
        (:`  `
          (`self.SoldierMove`))))))

(fn `UserConstructionScript`)